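; Demon pawn that spawns its default AI controller on BeginPlay and exposes its capsule hitbox and run radius through getters.
; StartDeath reads the AI blackboard: if the corrupted key is set, it flags the demon as caught instead of destroying it.
; Otherwise it clears corruption on the blackboard's nearest object via Object_IF and destroys itself, doing neither if that cast fails.
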(event EventBeginPlay
  (Pawn|SpawnDefaultController))

(event EventStartDeath
  (bind _output_get (Variables|Default|SetBlackboard (AI|GetBlackboard (AI|GetAIController (Pawn|GetController)))))
  (if (ScalableFloat|GetValueasBool _output_get (Variables|Default|GetCorruptedKeyName))
    (AI|Components|Blackboard|SetValueasBool (Variables|Default|GetBlackboard) (Variables|Default|GetCaughtKeyName) true)
    (else
      (bind _asobject_if (Utilities|Casting|CastToObject_IF (AI|Components|Blackboard|GetValueasObject _output_get (Variables|Default|GetNearestObjectKeyName))))
      (Default|SetCorrupted _asobject_if false)
      (Actor|DestroyActor))))

(fn ConstructionScript)

(fn GetHitbox
  (return (Variables|Collision|GetCapsuleComponent)))

(fn GetRunRadius
  (return (Variables|Default|GetRunRadius)))