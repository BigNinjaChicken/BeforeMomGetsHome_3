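; IntroCameraServer_BP runs an intro sequence that shows the IntroServer_UW widget and advances numbered scenes on Jump presses.
; The first scene uses a timeline to lerp all local player pawns from this actor's location to a CameraMoveSpot_BP.
; The second and third scenes only start their timelines, with no update logic.
; A DoOnce gates presses until StartCooldown, not called within this Blueprint, finishes its timer and resets it.
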(event Custom|StartCooldown
  (params (Time :type Float%20%28double-precision%29))
  (Components|Timeline|SetPlayRate (Variables|Default|GetSceneCooldown) (/ 1.0 Time))
  (Timeline|SceneCooldown PlayFromStart
    (:Finished
      (Utilities|FlowControl|DoOnce false) ; enters at Reset
    )))

(event Custom|MovePlayerMulti
  (params (NewLocation :type Vector))
  (for _index (range 0 (Class|GameplayStatics|GetNumLocalPlayerControllers))
    (Transformation|SetActorLocation (Game|Player|GetPlayerPawn _index) NewLocation false false)))

(event EventBeginPlay
  (bind _returnvalue (UserInterface|CreateWidget "/Game/GameContent/Frazier/GameManager/IntroServer_UW.IntroServer_UW_C"))
  (bind _output_get (Variables|Default|SetUW _returnvalue))
  (UserInterface|Viewport|AddtoViewport _output_get 0))

(event Input|ActionEvents|InputActionJump
  (params (Key :type Key%20Structure :default "None"))
  (:Pressed
    (Utilities|FlowControl|DoOnce false
      (:Completed
        (Math|Integer|IncrementInt (Variables|Default|GetSceneNumber)
          (:%20%20
            (Utilities|FlowControl|Sequence
              (:then_0
                (if (== (Variables|Default|GetSceneNumber) 1)
                  (Components|Timeline|SetPlayRate (Variables|Default|GetTimeline_0) (/ 1.0 5.0))
                  (Variables|Default|SetActorCurrentLocation (Transformation|GetActorLocation))
                  (bind _returnvalue (Actor|GetActorOfClass "/Game/GameContent/Frazier/GameManager/CameraMoveSpot_BP.CameraMoveSpot_BP_C"))
                  (Variables|Default|SetCameraMoveSpot _returnvalue)
                  (bind _time (Timeline|Timeline_0 PlayFromStart)
                    (:Update
                      (CallFunction|MovePlayerMulti (Math|Vector|Lerp(Vector) (Variables|Default|GetActorCurrentLocation) (Transformation|GetActorLocation (Variables|Default|GetCameraMoveSpot)) (/ _time 0.5)))))))
              (:then_1
                (if (== (Variables|Default|GetSceneNumber) 2)
                  (Components|Timeline|SetPlayRate (Variables|Default|GetTimeline_1) (/ 1.0 5.0))
                  (Timeline|Timeline_1 PlayFromStart)))
              (:then_2
                (if (== (Variables|Default|GetSceneNumber) 3)
                  (Components|Timeline|SetPlayRate (Variables|Default|GetTimeline_2) (/ 1.0 5.0))
                  (Timeline|Timeline_2 PlayFromStart))))))))))

(fn ConstructionScript)