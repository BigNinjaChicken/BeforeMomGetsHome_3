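; IntroCameraClient_BP is the client-side camera for the multiplayer intro, exposing its camera and driving the intro UI.
; On BeginPlay it caches the GameManager and, when running on the server, has player controller 0 possess IntroCameraServer_BP instead.
; SetUW adds an IntroMulti_UW widget to the viewport, and GetUW steps through its parts by index, showing one and collapsing the previous.
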(event EventBeginPlay
  (bind _returnvalue (Actor|GetActorOfClass "/Game/GameContent/Frazier/GameManager/GameManager.GameManager_C"))
  (Variables|Default|SetGameManager _returnvalue)
  (if (Networking|IsServer)
    (bind _returnvalue_2 (Actor|GetActorOfClass "/Game/GameContent/Frazier/GameManager/IntroCameraServer_BP.IntroCameraServer_BP_C"))
    (Pawn|Possess (Game|GetPlayerController 0) _returnvalue_2)))

(event EventSetUW
  (bind _returnvalue (UserInterface|CreateWidget "/Game/GameContent/Frazier/GameManager/IntroMulti_UW.IntroMulti_UW_C" (Game|GetPlayerController 0)))
  (bind _output_get (Variables|Default|SetUWMulti _returnvalue))
  (UserInterface|Viewport|AddtoViewport _output_get 0))

(fn ConstructionScript)

(fn GetCamera
  (return (Variables|Default|GetCamera)))

(fn GetUW
  (params (Index :type Integer))
  (Widget|SetVisibility (Utilities|Array|Get(acopy) (Variables|/Game/GameContent/Frazier/GameManager/IntroMulti_UW.IntroMulti_UW_C|GetAllParts (Variables|Default|GetUWMulti)) Index) "Visible")
  (if (!= Index 0)
    (Widget|SetVisibility (Utilities|Array|Get(acopy) (Variables|/Game/GameContent/Frazier/GameManager/IntroMulti_UW.IntroMulti_UW_C|GetAllParts (Variables|Default|GetUWMulti)) (- Index 1)) "Collapsed")
    (return)))