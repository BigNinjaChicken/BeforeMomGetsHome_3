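; Game manager that runs a timed round, spawning demons in phases and ending the game for every child character.
; StartGame stretches a timeline over RoundLength and copies its elapsed time to each ChildCharacter_BP.
; Hard-coded time windows set spawn count and interval, with the last window only printing a debug message.
; SpawnDemons picks random EnemySpawnSpots whose level is at or below the GameInstance's saved level.
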(event Custom|StartGame
  (Variables|Time|SetNextSpawnTime 0.0)
  (Components|Timeline|SetPlayRate (Variables|Default|GetGameTimerTimeline) (/ 1.0 (Variables|Time|GetRoundLength)))
  (bind _time (Timeline|GameTimerTimeline PlayFromStart)
    (:Update
      (bind _output_get (Variables|Time|SetTimer (* _time (Variables|Time|GetRoundLength))))
      (bind _outactors (Actor|GetAllActorsOfClass "/Game/GameContent/Frazier/InGameCharacter/ChildCharacter_BP.ChildCharacter_BP_C"))
      (for _array_element _outactors
        (Variables|/Game/GameContent/Frazier/InGameCharacter/ChildCharacter_BP.ChildCharacter_BP_C|SetChildTimer _array_element (Variables|Time|GetTimer)))
      (if (> _output_get (Variables|Time|GetNextSpawnTime))
        (Utilities|FlowControl|Sequence
          (:then_0
            (bind _returnvalue (CallFunction|IsTimerBetween 0.0 5.0))
            (if _returnvalue
              (CallFunction|SpawnDemons 2 5.0)))
          (:then_1
            (bind _returnvalue_2 (CallFunction|IsTimerBetween 5.1 25.0))
            (if _returnvalue_2
              (CallFunction|SpawnDemons 1 7.0)))
          (:then_2
            (bind _returnvalue_3 (CallFunction|IsTimerBetween 25.1 5e+01))
            (if _returnvalue_3
              (CallFunction|SpawnDemons 2 5.0)))
          (:then_3
            (bind _returnvalue_4 (CallFunction|IsTimerBetween 50.1 75.0))
            (if _returnvalue_4
              (CallFunction|SpawnDemons 1 4.0)))
          (:then_4
            (bind _returnvalue_5 (CallFunction|IsTimerBetween 75.1 9e+01))
            (if _returnvalue_5
              (Development|PrintString "Near End Of Round"))))))
    (:Finished
      (bind _outactors_2 (Actor|GetAllActorsOfClass "/Game/GameContent/Frazier/InGameCharacter/ChildCharacter_BP.ChildCharacter_BP_C"))
      (for _array_element_2 _outactors_2
        (Default|EndGameServer _array_element_2)))))

(fn ConstructionScript)

(fn IsTimerBetween
  (params (GreaterThan :type Float%20%28double-precision%29) (LessThan :type Float%20%28double-precision%29))
  (bind _timer (Variables|Time|GetTimer))
  (return (and (> _timer GreaterThan) (< _timer LessThan))))

(fn SpawnDemons
  (params (SpawnHowMany :type Integer) (NextSpawntime :type Float%20%28double-precision%29))
  (Utilities|Array|Clear (Variables|Default|GetAvaliableSpawnPoints))
  (bind _assaved_data_gi (Utilities|Casting|CastToSavedData_GI (Game|GetGameInstance)))
  (bind _outactors (Actor|GetAllActorsOfClass "/Game/GameContent/Frazier/GameManager/EnemySpawnSpot.EnemySpawnSpot_C"))
  (for _array_element _outactors
    (if (<= (Variables|/Game/GameContent/Frazier/GameManager/EnemySpawnSpot.EnemySpawnSpot_C|GetLevel _array_element) (Variables|/Game/GameContent/Frazier/GameManager/SavedData_GI.SavedData_GI_C|GetLevel _assaved_data_gi))
      (Utilities|Array|Add (Variables|Default|GetAvaliableSpawnPoints) _array_element)))
  (for _index (range 1 SpawnHowMany)
    (Game|SpawnActorfromClass "/Game/GameContent/Frazier/Demons/Demon_BP.Demon_BP_C" (Math|Transform|MakeTransform (Transformation|GetActorLocation (.OutItem (Utilities|Array|Random (Variables|Default|GetAvaliableSpawnPoints)))) "0, 0, 0" "1.000000,1.000000,1.000000") "Undefined" 0 0))
  (Variables|Time|SetNextSpawnTime (+ (Variables|Time|GetNextSpawnTime) NextSpawntime))
  (return))